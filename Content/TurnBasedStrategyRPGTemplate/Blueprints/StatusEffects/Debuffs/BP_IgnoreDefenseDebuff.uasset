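; Status effect debuff that reduces the affected character's defense to zero for as long as it lasts.
; On start it stores the character's current defense and applies the negated value as a stat change through ApplyStats.
; When the effect ends, it adds the stored amount back and destroys its own actor.
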(event `self.OnStatusEffectStarted`
  ;[1 1 1] Make defense 0 until the debuff ends
  (set `self.initialDefense` (`/Game/TurnBasedStrategyRPGTemplate/Blueprints/Units/Characters/BP_CharacterBase.currentDefense` (`self.affectedCharacter`)))
  (`/Game/TurnBasedStrategyRPGTemplate/Blueprints/Units/Characters/BP_CharacterBase.ApplyStats` (`self.affectedCharacter`) 0 (* (`self.initialDefense`) -1) 0 0 0 0))

(event `self.OnStatusEffectEnded`
  ;[1 1 1] Make defense 0 until the debuff ends
  (`/Game/TurnBasedStrategyRPGTemplate/Blueprints/Units/Characters/BP_CharacterBase.ApplyStats` (`self.affectedCharacter`) 0 (`self.initialDefense`) 0 0 0 0)
  (`self.K2_DestroyActor`))

(fn `UserConstructionScript`
  (`parent.UserConstructionScript`))