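; Base actor for buffs and debuffs on turn-based battle characters, with hooks for children and a helper for element-reduced DOT damage.
; On initialization it removes conflicting non-aura effects, then applies flat and MainStats-multiplied stat changes plus element reductions, negating them on removal.
; Timed effects count down on new turns; aura effects skip this, ending on aura refresh or when the affected character leaves its slot.
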(event `self.ReceiveBeginPlay`
  ;[1 1 1] Initialize status effect
  (if (not (`self.isFromAura`))
    (`self.PlaySound`)
    (`self.PlayParticleEffect`)))

(event `Initialize`
  (bind (_elementreductions_normal _elementreductions_fire _elementreductions_earth _elementreductions_air _elementreductions_water) (break `/Game/TurnBasedStrategyRPGTemplate/Blueprints/Structs/S_ElementReductions` (`self.elementReductions`)))
  (bind (_statadditions_attack _statadditions_defense _statadditions_mindamage _statadditions_maxdamage _statadditions_ammo _statadditions_movementrange) (break `/Game/TurnBasedStrategyRPGTemplate/Blueprints/Structs/S_CharacterStatBuff` (`self.statAdditions`)))
  ;[1 1 1] Initialize status effect
  (add `/Game/TurnBasedStrategyRPGTemplate/Blueprints/Units/Characters/BP_CharacterBase.OnDead` (`self.affectedCharacter`) (delegate `OnCharacterDies`))
  (add `/Game/TurnBasedStrategyRPGTemplate/Blueprints/Core/BP_BattleController.OnNewTurn` (`/Game/TurnBasedStrategyRPGTemplate/Blueprints/Units/Characters/BP_CharacterBase.battleController` (`self.affectedCharacter`)) (delegate `OnNewTurnHandler`))
  (`self.SetAuraLogic`)
  (`self.RemoveOtherStatusEffects`)
  (`self.ApplyStats` (`KismetMathLibrary.FTrunc` _statadditions_attack) (`KismetMathLibrary.FTrunc` _statadditions_defense) (`KismetMathLibrary.FTrunc` _statadditions_mindamage) (`KismetMathLibrary.FTrunc` _statadditions_maxdamage) (`KismetMathLibrary.FTrunc` _statadditions_ammo) (`KismetMathLibrary.FTrunc` _statadditions_movementrange))
  (bind _multipliedstats (`self.GetMultipliedStats`))
  (`self.ApplyStats` (`.attack_4_070694DD47F26EDC2721E9A1E54F07AC` (break `/Game/TurnBasedStrategyRPGTemplate/Blueprints/Structs/S_CharacterStats` _multipliedstats)) (`.defense_6_A8FC241645B1DBC0E19D38A28BC31C2B` (break `/Game/TurnBasedStrategyRPGTemplate/Blueprints/Structs/S_CharacterStats` _multipliedstats)) (`.minDamage_8_CC77DE244DFC375E9B688F870C3B4048` (break `/Game/TurnBasedStrategyRPGTemplate/Blueprints/Structs/S_CharacterStats` _multipliedstats)) (`.maxDamage_10_A27D6D794D2F0CF68426F3B2A36C6B81` (break `/Game/TurnBasedStrategyRPGTemplate/Blueprints/Structs/S_CharacterStats` _multipliedstats)) (`.ammo_14_444ED39342AC484F3DFA0793A68D51C1` (break `/Game/TurnBasedStrategyRPGTemplate/Blueprints/Structs/S_CharacterStats` _multipliedstats)) (`.movementRange_12_C21832B24A6A4E756F34C497589017A0` (break `/Game/TurnBasedStrategyRPGTemplate/Blueprints/Structs/S_CharacterStats` _multipliedstats)))
  (`self.ApplyElementReductions` _elementreductions_normal _elementreductions_fire _elementreductions_earth _elementreductions_air _elementreductions_water)
  (`self.OnStatusEffectStarted`))

(event `OnCharacterDies`
  (params (character :type "/Game/TurnBasedStrategyRPGTemplate/Blueprints/Units/Characters/BP_CharacterBase Object Reference"))
  ;[1 1 1] Initialize status effect
  (`self.K2_DestroyActor`))

(event `OnNewTurnHandler`
  (params (newTurn :type Integer))
  ;[1 1 1] Initialize status effect
  (if (not (`self.isFromAura`))
    (bind _result (`/Engine/EditorBlueprintResources/StandardMacros.DecrementInt` (`self.turnDuration`))
      (:`  `
        (`self.OnTurnDurationUpdated`)
        (if (<= _result 0)
          (`self.RemoveStatusEffect`))))))

(event `SetAuraLogic`
  ;[1 1 1] Remove status effect when the caster is dead / moved if it is from aura
  (if (and (`self.isFromAura`) (!= (`self.affectedCharacter`) (`self.casterCharacter`)))
    (add `/Game/TurnBasedStrategyRPGTemplate/Blueprints/Units/Characters/BP_CharacterBase.OnRefreshAuras` (`self.casterCharacter`) (delegate `OnRefreshAurasHandler`))
    (add `/Game/TurnBasedStrategyRPGTemplate/Blueprints/Units/Characters/BP_CharacterBase.OnCharacterRemovedFromSlot` (`self.affectedCharacter`) (delegate `OnCasterCharacterRemovedFromSlot`))))

(event `OnRefreshAurasHandler`
  ;[1 1 1] Remove status effect when the caster is dead / moved if it is from aura
  (`self.RemoveStatusEffect`)
  (`/Game/TurnBasedStrategyRPGTemplate/Blueprints/Units/Characters/BP_CharacterBase.ReceiveAuras` (`self.affectedCharacter`)))

(event `OnCasterCharacterRemovedFromSlot`
  (params (character :type "/Game/TurnBasedStrategyRPGTemplate/Blueprints/Units/Characters/BP_CharacterBase Object Reference"))
  ;[1 1 1] Remove status effect when the caster is dead / moved if it is from aura
  (`self.RemoveStatusEffect`))

(event `RemoveOtherStatusEffects`
  ;[1 1 1] Remove other status effects that are not from aura
  (bind _allstatuseffects (`self.GetAllStatusEffects`))
  (bind (_arrayindex _arrayelement) (`/Engine/EditorBlueprintResources/StandardMacros.ReverseForEachLoop` _allstatuseffects)
    (:`LoopBody`
      (if (and (`KismetArrayLibrary.Array_Contains` (`self.removesStatusEffects`) (`GameplayStatics.GetObjectClass` _arrayelement)) (not (`/Game/TurnBasedStrategyRPGTemplate/Blueprints/StatusEffects/BP_StatusEffectBase.isFromAura` _arrayelement)) (not (`self.isFromAura`)))
        (`self.RemoveStatusEffect` _arrayelement)))))

(event `ApplyStats`
  (params (attack :type Integer) (defense :type Integer) (minDamage :type Integer) (maxDamage :type Integer) (ammo :type Integer) (movementRange :type Integer))
  ;[1 1 1] Apply buff stats
  (`/Game/TurnBasedStrategyRPGTemplate/Blueprints/Units/Characters/BP_CharacterBase.ApplyStats` (`self.affectedCharacter`) attack defense minDamage maxDamage ammo movementRange))

(event `ApplyElementReductions`
  (params (normalReduction :type "Float (double-precision)") (fireReduction :type "Float (double-precision)") (currentEarthReduction :type "Float (double-precision)") (currentAirReduction :type "Float (double-precision)") (currentWaterReduction :type "Float (double-precision)"))
  ;[1 1 1] Apply element reductions
  (`/Game/TurnBasedStrategyRPGTemplate/Blueprints/Units/Characters/BP_CharacterBase.ApplyElementReductions` (`self.affectedCharacter`) normalReduction fireReduction currentEarthReduction currentAirReduction currentWaterReduction))

(event `RemoveStats`
  (bind (_statadditions_attack _statadditions_defense _statadditions_mindamage _statadditions_maxdamage _statadditions_ammo _statadditions_movementrange) (break `/Game/TurnBasedStrategyRPGTemplate/Blueprints/Structs/S_CharacterStatBuff` (`self.statAdditions`)))
  ;[1 1 1] Remove stats
  (`self.ApplyStats` (* (`KismetMathLibrary.FTrunc` _statadditions_attack) -1) (* (`KismetMathLibrary.FTrunc` _statadditions_defense) -1) (* (`KismetMathLibrary.FTrunc` _statadditions_mindamage) -1) (* (`KismetMathLibrary.FTrunc` _statadditions_maxdamage) -1) (* (`KismetMathLibrary.FTrunc` _statadditions_ammo) -1) (* (`KismetMathLibrary.FTrunc` _statadditions_movementrange) -1))
  (bind _multipliedstats (`self.GetMultipliedStats`))
  (`self.ApplyStats` (* (`.attack_4_070694DD47F26EDC2721E9A1E54F07AC` (break `/Game/TurnBasedStrategyRPGTemplate/Blueprints/Structs/S_CharacterStats` _multipliedstats)) -1) (* (`.defense_6_A8FC241645B1DBC0E19D38A28BC31C2B` (break `/Game/TurnBasedStrategyRPGTemplate/Blueprints/Structs/S_CharacterStats` _multipliedstats)) -1) (* (`.minDamage_8_CC77DE244DFC375E9B688F870C3B4048` (break `/Game/TurnBasedStrategyRPGTemplate/Blueprints/Structs/S_CharacterStats` _multipliedstats)) -1) (* (`.maxDamage_10_A27D6D794D2F0CF68426F3B2A36C6B81` (break `/Game/TurnBasedStrategyRPGTemplate/Blueprints/Structs/S_CharacterStats` _multipliedstats)) -1) (* (`.ammo_14_444ED39342AC484F3DFA0793A68D51C1` (break `/Game/TurnBasedStrategyRPGTemplate/Blueprints/Structs/S_CharacterStats` _multipliedstats)) -1) (* (`.movementRange_12_C21832B24A6A4E756F34C497589017A0` (break `/Game/TurnBasedStrategyRPGTemplate/Blueprints/Structs/S_CharacterStats` _multipliedstats)) -1)))

(event `RemoveElementReductions`
  (bind (_elementreductions_normal _elementreductions_fire _elementreductions_earth _elementreductions_air _elementreductions_water) (break `/Game/TurnBasedStrategyRPGTemplate/Blueprints/Structs/S_ElementReductions` (`self.elementReductions`)))
  ;[1 1 1] Remove element reductions
  (`self.ApplyElementReductions` (* _elementreductions_normal -1.0) (* _elementreductions_fire -1.0) (* _elementreductions_earth -1.0) (* _elementreductions_air -1.0) (* _elementreductions_water -1.0)))

(event `OnStatusEffectStarted`
  ;[1 1 1] Override in child blueprints
)

(event `OnStatusEffectEnded`
  ;[1 1 1] Override in child blueprints
  (`self.K2_DestroyActor`))

(event `RemoveFromCharacter`
  ;[1 1 1] Override in child blueprints
)

(event `OnDOT`
  ;[1 1 1] Override in child blueprints
  (`self.OnDOTApplied` 0.0))

(event `RemoveStatusEffect`
  ;[1 1 1] Remove status effect
  (`self.RemoveStats`)
  (`self.RemoveElementReductions`)
  (`self.RemoveFromCharacter`)
  (`self.OnStatusEffectEnded`))

(event `PlayParticleEffect`
  ;[1 1 1] Spawn particle effect
  (`/Engine/EditorBlueprintResources/StandardMacros.IsValid` (`self.particleEffect`)
    (:`Is Valid`
      (`GameplayStatics.SpawnEmitterAtLocation` (`self.particleEffect`) (`SceneComponent.K2_GetComponentLocation` (`/Game/TurnBasedStrategyRPGTemplate/Blueprints/Units/Characters/BP_CharacterBase.ProjectileHitLocation` (`self.affectedCharacter`)))))
    (:`Is Not Valid`
      (`/Engine/EditorBlueprintResources/StandardMacros.IsValid` (`self.niagaraParticleEffect`)
        (:`Is Valid`
          (`NiagaraFunctionLibrary.SpawnSystemAtLocation` (`self.niagaraParticleEffect`) (`SceneComponent.K2_GetComponentLocation` (`/Game/TurnBasedStrategyRPGTemplate/Blueprints/Units/Characters/BP_CharacterBase.ProjectileHitLocation` (`self.affectedCharacter`)))))))))

(event `PlaySound`
  (bind _sound (`self.sound`))
  ;[1 1 1] Play sound
  (`/Engine/EditorBlueprintResources/StandardMacros.IsValid` _sound
    (:`Is Valid`
      (`GameplayStatics.PlaySound2D` _sound 1.0 1.0 0.0 null null))))

(fn `GetAllStatusEffects`
  (returns (allStatusEffects :type "Array of /Game/TurnBasedStrategyRPGTemplate/Blueprints/StatusEffects/BP_StatusEffectBase Object Reference"))
  (locals (currentAllStatusEffects :type "Array of /Game/TurnBasedStrategyRPGTemplate/Blueprints/StatusEffects/BP_StatusEffectBase Object Reference"))
  ;[1 1 1] Returns all status effects
  (`KismetArrayLibrary.Array_Append` (`local.currentAllStatusEffects`) (`/Game/TurnBasedStrategyRPGTemplate/Blueprints/Units/Characters/BP_CharacterBase.currentBuffs` (`self.affectedCharacter`)))
  (`KismetArrayLibrary.Array_Append` (`local.currentAllStatusEffects`) (`/Game/TurnBasedStrategyRPGTemplate/Blueprints/Units/Characters/BP_CharacterBase.currentDebuffs` (`self.affectedCharacter`)))
  (return (`local.currentAllStatusEffects`)))

(fn `GetDamageAfterElementReductions`
  (params (damage :type Integer) (element :type "/Game/TurnBasedStrategyRPGTemplate/Blueprints/Enums/E_Element Enum" :default "NewEnumerator0"))
  (returns (finalDamage :type Integer))
  (bind _affectedcharacter (`self.affectedCharacter`))
  ;[1 1 1] Reduce element damage for DOT status effects
  (return (`KismetMathLibrary.Max` (- damage (`KismetMathLibrary.FTrunc` (* damage (`KismetMathLibrary.FClamp` (select `/Game/TurnBasedStrategyRPGTemplate/Blueprints/Enums/E_Element` element :`NewEnumerator0` (`/Game/TurnBasedStrategyRPGTemplate/Blueprints/Units/Characters/BP_CharacterBase.currentNormalReduction` _affectedcharacter) :`NewEnumerator1` (`/Game/TurnBasedStrategyRPGTemplate/Blueprints/Units/Characters/BP_CharacterBase.currentFireReduction` _affectedcharacter) :`NewEnumerator2` (`/Game/TurnBasedStrategyRPGTemplate/Blueprints/Units/Characters/BP_CharacterBase.currentEarthReduction` _affectedcharacter) :`NewEnumerator3` (`/Game/TurnBasedStrategyRPGTemplate/Blueprints/Units/Characters/BP_CharacterBase.currentAirReduction` _affectedcharacter) :`NewEnumerator4` (`/Game/TurnBasedStrategyRPGTemplate/Blueprints/Units/Characters/BP_CharacterBase.currentWaterReduction` _affectedcharacter)) -1.0)))))))

(fn `GetMultipliedStats`
  (returns (multipliedStats :type "/Game/TurnBasedStrategyRPGTemplate/Blueprints/Structs/S_CharacterStats Structure"))
  (bind (_statmultiplications_attack _statmultiplications_defense _statmultiplications_mindamage _statmultiplications_maxdamage _statmultiplications_ammo _statmultiplications_movementrange) (break `/Game/TurnBasedStrategyRPGTemplate/Blueprints/Structs/S_CharacterStatBuff` (`self.statMultiplications`)))
  (bind (_mainstats_maxhealth _mainstats_attack _mainstats_defense _mainstats_mindamage _mainstats_maxdamage _mainstats_ammo _mainstats_movementrange) (break `/Game/TurnBasedStrategyRPGTemplate/Blueprints/Structs/S_CharacterStats` (`/Game/TurnBasedStrategyRPGTemplate/Blueprints/Units/Characters/BP_CharacterBase.mainStats` (`self.affectedCharacter`))))
  ;[1 1 1] Return multiplied stats
  (return (make `/Game/TurnBasedStrategyRPGTemplate/Blueprints/Structs/S_CharacterStats` 0 (`KismetMathLibrary.FFloor` (* _mainstats_attack _statmultiplications_attack)) (`KismetMathLibrary.FFloor` (* _mainstats_defense _statmultiplications_defense)) (`KismetMathLibrary.FFloor` (* _mainstats_mindamage _statmultiplications_mindamage)) (`KismetMathLibrary.FFloor` (* _mainstats_maxdamage _statmultiplications_maxdamage)) (`KismetMathLibrary.FFloor` (* _mainstats_ammo _statmultiplications_ammo)) (`KismetMathLibrary.FFloor` (* _mainstats_movementrange _statmultiplications_movementrange)))))

(fn `ShowElementOnUI`
  (returns (NewParam :type "/Game/TurnBasedStrategyRPGTemplate/Blueprints/Enums/E_Element Enum"))
  ;[1 1 1] Shows element color and image on UI
  (return "NewEnumerator0"))

(fn `UserConstructionScript`)