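; Short-lived helper actor that animates one battle queue UI entry shifting to the position and scale of a target entry.
; Shift captures both widgets' transforms, converting the target's absolute position into the moving widget's local space, then runs a speed-scaled Timeline to lerp between them.
; An entry leaving the front of the queue follows a height curve that arcs it upward.
; The actor destroys itself when finished, or immediately if either index falls outside the first twelve slots.
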(event `Shift`
  (params (battleQueueUI :type "/Game/TurnBasedStrategyRPGTemplate/Blueprints/Widgets/WBP_BattleQueueCharacterUI Object Reference") (targetBattleQueueUI :type "/Game/TurnBasedStrategyRPGTemplate/Blueprints/Widgets/WBP_BattleQueueCharacterUI Object Reference") (shiftFromIndex :type Integer) (shiftToIndex :type Integer))
  (bind (_targetlocation_x _targetlocation_y) (`KismetMathLibrary.BreakVector2D` (`self.targetLocation`)))
  (bind _currentui (`self.currentUI`))
  (bind _targetlocation_x_2 (`KismetMathLibrary.BreakVector2D` (`self.targetLocation`)))
  (bind (_startlocation_x _startlocation_y) (`KismetMathLibrary.BreakVector2D` (`self.startLocation`)))
  (bind (_returnvalue_x _returnvalue_y) (`KismetMathLibrary.BreakVector2D` (`SlateBlueprintLibrary.LocalToAbsolute` (`Widget.GetCachedGeometry` (`/Game/TurnBasedStrategyRPGTemplate/Blueprints/Widgets/WBP_BattleQueueCharacterUI.LocationOverlay` (`self.targetUI`))) (0.0 0.0))))
  ;[1 1 1] Shifts the battle queue UI to target location
  (set `self.currentUI` battleQueueUI)
  (set `self.targetUI` targetBattleQueueUI)
  (set `self.shiftFromIndex` shiftFromIndex)
  (set `self.shiftToIndex` shiftToIndex)
  (`self.targetUI`
    (:`then`
      (set `self.startTransform` (`Widget.RenderTransform` (`/Game/TurnBasedStrategyRPGTemplate/Blueprints/Widgets/WBP_BattleQueueCharacterUI.Container` _currentui)))
      (set `self.startLocation` (`CanvasPanelSlot.GetPosition` (`WidgetLayoutLibrary.SlotAsCanvasSlot` (`/Game/TurnBasedStrategyRPGTemplate/Blueprints/Widgets/WBP_BattleQueueCharacterUI.LocationOverlay` _currentui))))
      (set `self.targetTransform` (`Widget.RenderTransform` (`/Game/TurnBasedStrategyRPGTemplate/Blueprints/Widgets/WBP_BattleQueueCharacterUI.Container` (`self.targetUI`))))
      (set `self.targetLocation` (`SlateBlueprintLibrary.AbsoluteToLocal` (`Widget.GetCachedGeometry` (`/Game/TurnBasedStrategyRPGTemplate/Blueprints/Widgets/WBP_BattleQueueCharacterUI.LocationOverlay` (`self.currentUI`))) (`KismetMathLibrary.MakeVector2D` _returnvalue_x _returnvalue_y)))
      (`TimelineComponent.SetPlayRate` (`self.MoveOverTime`) (/ 1.0 (`self.lerpSpeed`)))
      (if (and (< (`self.shiftFromIndex`) 12) (< (`self.shiftToIndex`) 12))
        (bind (_direction _alpha _height) (`Timeline|MoveOverTime` :!via `PlayFromStart`)
          (:`Update`
            (`CanvasPanelSlot.SetPosition` (`WidgetLayoutLibrary.SlotAsCanvasSlot` (`/Game/TurnBasedStrategyRPGTemplate/Blueprints/Widgets/WBP_BattleQueueCharacterUI.LocationOverlay` (`self.currentUI`))) (`KismetMathLibrary.MakeVector2D` (`KismetMathLibrary.Lerp` _startlocation_x _targetlocation_x_2 _alpha) (`KismetMathLibrary.Lerp` _startlocation_y (select `bool` (and (== (`self.shiftFromIndex`) 0) (!= (`self.shiftToIndex`) 0)) :`false` _targetlocation_y :`true` (+ (* -300 _height) _targetlocation_y)) _alpha)))
            (bind _returnvalue (`KismetMathLibrary.Lerp` (`KismetMathLibrary.BreakVector2D` (`.Scale` (break `WidgetTransform` (`self.startTransform`)))) (`KismetMathLibrary.BreakVector2D` (`.Scale` (break `WidgetTransform` (`self.targetTransform`)))) _alpha))
            (`Widget.SetRenderScale` (`/Game/TurnBasedStrategyRPGTemplate/Blueprints/Widgets/WBP_BattleQueueCharacterUI.Container` (`self.currentUI`)) (`KismetMathLibrary.MakeVector2D` _returnvalue _returnvalue)))
          (:`Finished`
            (`self.K2_DestroyActor` :!label _label)))
        (else
          (goto _label))))
    (:`else`)))

(fn `UserConstructionScript`)