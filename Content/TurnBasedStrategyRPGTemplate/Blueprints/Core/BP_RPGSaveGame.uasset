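; BP_RPGSaveGame is a save game container for hero progress in the turn-based strategy RPG template.
; It stores experience, gold, current mana, the player character list, explore hero, active and completed quests, backpack and equipment.
; SaveHero copies all these values into its variables in one call, and LoadHero returns them together.
; It holds only data, with no disk read or write logic.
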(event `SaveHero`
  (params (exp :type Integer) (gold :type Integer) (currentMana :type Integer) (playerCharacterList :type "Array of /Game/TurnBasedStrategyRPGTemplate/Blueprints/Structs/S_PlayerCharacterData Structure") (exploreHero :type "/Game/TurnBasedStrategyRPGTemplate/Blueprints/Heroes/Explore/BP_ExploreHeroBase Class Reference") (activeQuestData :type "Map of /Game/TurnBasedStrategyRPGTemplate/Blueprints/Quests/BP_QuestBase Class Reference to /Game/TurnBasedStrategyRPGTemplate/Blueprints/Structs/S_QuestStepData Structure") (completedQuestData :type "Map of /Game/TurnBasedStrategyRPGTemplate/Blueprints/Quests/BP_QuestBase Class Reference to Integer") (backpack :type "Array of /Game/TurnBasedStrategyRPGTemplate/Blueprints/Equipments/BP_EquipmentBase Class Reference") (equipment :type "Array of /Game/TurnBasedStrategyRPGTemplate/Blueprints/Equipments/BP_EquipmentBase Class Reference"))
  ;[1 1 1] Save hero variables
  (set `self.exp` exp)
  (set `self.gold` gold)
  (set `self.currentMana` currentMana)
  (set `self.playerCharacterList` playerCharacterList)
  (set `self.exploreHero` exploreHero)
  (set `self.activeQuestData` activeQuestData)
  (set `self.completedQuestData` completedQuestData)
  (set `self.backpack` backpack)
  (set `self.equipment` equipment))

(fn `LoadHero`
  (returns (exp :type Integer) (gold :type Integer) (currentMana :type Integer) (playerCharacterList :type "Array of /Game/TurnBasedStrategyRPGTemplate/Blueprints/Structs/S_PlayerCharacterData Structure") (exploreHero :type "/Game/TurnBasedStrategyRPGTemplate/Blueprints/Heroes/Explore/BP_ExploreHeroBase Class Reference") (activeQuestData :type "Map of /Game/TurnBasedStrategyRPGTemplate/Blueprints/Quests/BP_QuestBase Class Reference to /Game/TurnBasedStrategyRPGTemplate/Blueprints/Structs/S_QuestStepData Structure") (completedQuestData :type "Map of /Game/TurnBasedStrategyRPGTemplate/Blueprints/Quests/BP_QuestBase Class Reference to Integer") (backpack :type "Array of /Game/TurnBasedStrategyRPGTemplate/Blueprints/Equipments/BP_EquipmentBase Class Reference") (equipment :type "Array of /Game/TurnBasedStrategyRPGTemplate/Blueprints/Equipments/BP_EquipmentBase Class Reference"))
  ;[1 1 1] Load hero variables
  (return (`self.exp`) (`self.gold`) (`self.currentMana`) (`self.playerCharacterList`) (`self.exploreHero`) (`self.activeQuestData`) (`self.completedQuestData`) (`self.backpack`) (`self.equipment`)))