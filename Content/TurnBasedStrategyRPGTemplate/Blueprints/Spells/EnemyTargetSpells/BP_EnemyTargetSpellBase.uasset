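; Base Blueprint for spells that target an enemy unit in the turn-based strategy RPG.
; Enabling or disabling the spell notifies the BattleController's Grid to switch enemy targeting on or off.
; A setter stores the target slot, and GetSpellSlots adds that slot's contained character to CurrentEnemies without duplicates.
; It returns that list without clearing it, or returns it unchanged when the slot is invalid.
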(event `self.OnSpellEnabled`
  ;[1 1 1] Enable / disable ally target spell
  (`/Game/TurnBasedStrategyRPGTemplate/Blueprints/Grid/BP_Grid.OnEnemyTargetSpellEnabled` (`/Game/TurnBasedStrategyRPGTemplate/Blueprints/Core/BP_BattleController.grid` (`self.battleController`))))

(event `self.OnSpellDisabled`
  ;[1 1 1] Enable / disable ally target spell
  (`/Game/TurnBasedStrategyRPGTemplate/Blueprints/Grid/BP_Grid.OnEnemyTargetSpellDisabled` (`/Game/TurnBasedStrategyRPGTemplate/Blueprints/Core/BP_BattleController.grid` (`self.battleController`))))

(event `self.SetTargetSlot`
  (params (slot :type "/Game/TurnBasedStrategyRPGTemplate/Blueprints/Grid/Slots/BP_SlotBase Object Reference"))
  ;[1 1 1] Set target slot for the spell
  (set `self.targetSlot` slot))

(fn `GetSpellSlots`
  (returns (slotsInRange :type "Array of /Game/TurnBasedStrategyRPGTemplate/Blueprints/Grid/Slots/BP_SlotBase Object Reference") (emptySlots :type "Array of /Game/TurnBasedStrategyRPGTemplate/Blueprints/Grid/Slots/BP_SlotBase Object Reference") (allies :type "Array of /Game/TurnBasedStrategyRPGTemplate/Blueprints/Units/Characters/BP_CharacterBase Object Reference") (enemies :type "Array of /Game/TurnBasedStrategyRPGTemplate/Blueprints/Units/Characters/BP_CharacterBase Object Reference"))
  (locals (currentEnemies :type "Array of /Game/TurnBasedStrategyRPGTemplate/Blueprints/Units/Characters/BP_CharacterBase Object Reference"))
  ;[1 1 1] Return enemies in target slot
  (`/Engine/EditorBlueprintResources/StandardMacros.IsValid` (`self.targetSlot`)
    (:`Is Valid`
      (`KismetArrayLibrary.Array_AddUnique` (`local.currentEnemies`) (cast `/Game/TurnBasedStrategyRPGTemplate/Blueprints/Units/Characters/BP_CharacterBase` (`/Game/TurnBasedStrategyRPGTemplate/Blueprints/Grid/Slots/BP_SlotBase.containedUnit` (`self.targetSlot`)) :!pure true))
      (return _ _ _ (`local.currentEnemies`)))
    (:`Is Not Valid`
      (return _ _ _ (`local.currentEnemies`)))))

(fn `UserConstructionScript`
  (`parent.UserConstructionScript`))