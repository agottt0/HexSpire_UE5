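; Meteor shower instant-cast spell for turn-based combat that damages all enemies passed to it, scaled by the hero's power stat.
; On use, it builds per-target damage data from a flat base plus power, then launches a fireball projectile from above at each enemy's hit location.
; Only the last projectile's hit event is bound; when it fires, all targets take damage at once and the spell ends.
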(event `self.OnSpellUsed`
  (params (emptySlots :type "Array of /Game/TurnBasedStrategyRPGTemplate/Blueprints/Grid/Slots/BP_SlotBase Object Reference (by ref)") (allies :type "Array of /Game/TurnBasedStrategyRPGTemplate/Blueprints/Units/Characters/BP_CharacterBase Object Reference (by ref)") (enemies :type "Array of /Game/TurnBasedStrategyRPGTemplate/Blueprints/Units/Characters/BP_CharacterBase Object Reference (by ref)"))
  ;[1 1 1] Damage all enemies (20 + hero's power stat)
  (bind _damagedata (`self.GetSpellDamage` enemies))
  (for _array_element enemies
    (bind _returnvalue (`SceneComponent.K2_GetComponentLocation` (`/Game/TurnBasedStrategyRPGTemplate/Blueprints/Units/Characters/BP_CharacterBase.ProjectileHitLocation` _array_element)))
    (bind _returnvalue_2 (`|SpawnActorFromClass` "/Game/TurnBasedStrategyRPGTemplate/Blueprints/Projectiles/BP_Fireball.BP_Fireball_C" (`KismetMathLibrary.MakeTransform` (+ _returnvalue (-400.0 0.0 600.0))) "Undefined" "OverrideRootScale" null null))
    (`/Game/TurnBasedStrategyRPGTemplate/Blueprints/Projectiles/BP_ProjectileBase.MoveProjectileToTarget` _returnvalue_2 _returnvalue)
    (set `self.lastMeteorProjectile` _returnvalue_2))
  (add `/Game/TurnBasedStrategyRPGTemplate/Blueprints/Projectiles/BP_ProjectileBase.OnProjectileHit` (`self.lastMeteorProjectile`) (delegate `OnLastMeteorProjectileHit`)))

(event `OnLastMeteorProjectileHit`
  ;[1 1 1] Damage all enemies (20 + hero's power stat)
  (remove `/Game/TurnBasedStrategyRPGTemplate/Blueprints/Projectiles/BP_ProjectileBase.OnProjectileHit` (`self.lastMeteorProjectile`) (delegate `OnLastMeteorProjectileHit`))
  (`self.DamageTargets` (stale `self.OnSpellUsed` _damagedata))
  (`self.EndSpell`))

(fn `GetSpellDamage`
  (params (targetCharacters :type "Array of /Game/TurnBasedStrategyRPGTemplate/Blueprints/Units/Characters/BP_CharacterBase Object Reference (by ref)"))
  (returns (damageData :type "Map of /Game/TurnBasedStrategyRPGTemplate/Blueprints/Units/Characters/BP_CharacterBase Object Reference to /Game/TurnBasedStrategyRPGTemplate/Blueprints/Structs/S_DamageData Structure"))
  (locals (currentDamageData :type "Map of /Game/TurnBasedStrategyRPGTemplate/Blueprints/Units/Characters/BP_CharacterBase Object Reference to /Game/TurnBasedStrategyRPGTemplate/Blueprints/Structs/S_DamageData Structure"))
  (bind _currentdamagedata (`local.currentDamageData`))
  (bind (_herostats_attack _herostats_defense _herostats_power) (break `/Game/TurnBasedStrategyRPGTemplate/Blueprints/Structs/S_HeroStats` (`/Game/TurnBasedStrategyRPGTemplate/Blueprints/Heroes/Battle/BP_BattleHeroBase.heroStats` (`self.hero`))))
  (bind _returnvalue (+ _herostats_power 20))
  ;[1 1 1] Return damage details
  (for _array_element targetCharacters
    (`BlueprintMapLibrary.Map_Add` _currentdamagedata _array_element (make `/Game/TurnBasedStrategyRPGTemplate/Blueprints/Structs/S_DamageData` _returnvalue _returnvalue _returnvalue 1.0 (`self.element`))))
  (return _currentdamagedata))

(fn `UserConstructionScript`
  (`parent.UserConstructionScript`))