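; Base spell actor for turn-based combat, with stubs for child spells to define targeting and damage.
; Casting reports mana cost, plays a montage chosen by hero class, and uses hero callbacks to trigger effects and completion, firing immediately without a montage.
; By default it applies buffs to living allies and debuffs to living enemies, replacing duplicates only with longer-lasting ones.
; A damage helper applies elemental reduction through the BattleController.
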(event `OnSpellEnabled`
  ;[1 1 1] Enable / disable spell
)

(event `OnSpellDisabled`
  ;[1 1 1] Enable / disable spell
)

(event `PlaySpellAnimation`
  ;[1 1 1] Play spell animation
  (set `self.animationHasEnded` false)
  (set `self.spellUsed` false)
  (`/Game/TurnBasedStrategyRPGTemplate/Blueprints/Heroes/Battle/BP_BattleHeroBase.OnSpellUsed` (`self.hero`) (`self.manaCost`))
  (`self.OnSpellUseStarted`)
  (`/Engine/EditorBlueprintResources/StandardMacros.IsValid` (`BlueprintMapLibrary.Map_Find` (`self.useSpellMontage`) (`GameplayStatics.GetObjectClass` (`self.hero`)))
    (:`Is Valid`
      (add `/Game/TurnBasedStrategyRPGTemplate/Blueprints/Heroes/Battle/BP_BattleHeroBase.OnSpellCasted` (`self.hero`) (delegate `OnSpellCastedHandler`))
      (add `/Game/TurnBasedStrategyRPGTemplate/Blueprints/Heroes/Battle/BP_BattleHeroBase.OnAnimationEnded` (`self.hero`) (delegate `OnAnimationEndedHandler`))
      (`/Game/TurnBasedStrategyRPGTemplate/Blueprints/Heroes/Battle/BP_BattleHeroBase.PlayAnimationMontage` (`self.hero`) (`BlueprintMapLibrary.Map_Find` (`self.useSpellMontage`) (`GameplayStatics.GetObjectClass` (`self.hero`)))))
    (:`Is Not Valid`
      (`self.OnAnimationPlayed`)
      (`self.OnAnimationEndedHandler`))))

(event `OnSpellCastedHandler`
  ;[1 1 1] Play spell animation
  (`self.OnAnimationPlayed`))

(event `OnAnimationEndedHandler`
  ;[1 1 1] Play spell animation
  (`/Game/TurnBasedStrategyRPGTemplate/Blueprints/Heroes/Battle/BP_BattleHeroBase.ClearSpellCallback` (`self.hero`))
  (`KismetSystemLibrary.Delay` (`self.spellAnimationDelay`))
  (if (`self.spellUsed`)
    (`self.OnSpellUseEnded`)
    (else
      (set `self.animationHasEnded` true))))

(event `OnAnimationPlayed`
  ;[1 1 1] Apply buff / debuff
  (bind (_slotsinrange _emptyslots _allies _enemies) (`self.GetSpellSlots`))
  (`self.OnSpellUsed` _emptyslots _allies _enemies))

(event `OnSpellUsed`
  (params (emptySlots :type "Array of /Game/TurnBasedStrategyRPGTemplate/Blueprints/Grid/Slots/BP_SlotBase Object Reference") (allies :type "Array of /Game/TurnBasedStrategyRPGTemplate/Blueprints/Units/Characters/BP_CharacterBase Object Reference") (enemies :type "Array of /Game/TurnBasedStrategyRPGTemplate/Blueprints/Units/Characters/BP_CharacterBase Object Reference"))
  ;[1 1 1] Apply buff / debuff
  (set `self.spellUsed` true)
  (bind _keys (`BlueprintMapLibrary.Map_Keys` (`self.buffs`)))
  (for _array_element _keys
    (for _array_element_2 allies
      (bind _isdead (`/Game/TurnBasedStrategyRPGTemplate/Blueprints/Units/Characters/BP_CharacterBase.IsDead` _array_element_2))
      (if (not _isdead)
        (`self.AddBuff` _array_element_2 _array_element (`BlueprintMapLibrary.Map_Find` (`self.buffs`) _array_element)))))
  (bind _keys_2 (`BlueprintMapLibrary.Map_Keys` (`self.debuffs`)))
  (for _array_element_3 _keys_2
    (for _array_element_4 enemies
      (bind _isdead_2 (`/Game/TurnBasedStrategyRPGTemplate/Blueprints/Units/Characters/BP_CharacterBase.IsDead` _array_element_4))
      (if (not _isdead_2)
        (`self.AddDebuff` _array_element_4 _array_element_3 (`BlueprintMapLibrary.Map_Find` (`self.debuffs`) _array_element_3))))))

(event `AddBuff`
  (params (affectedCharacter :type "/Game/TurnBasedStrategyRPGTemplate/Blueprints/Units/Characters/BP_CharacterBase Object Reference") (buff :type "/Game/TurnBasedStrategyRPGTemplate/Blueprints/StatusEffects/Buffs/BP_BuffBase Class Reference") (turnDuration :type Integer))
  ;[1 1 1] Add buff / debuff
  (bind _returnvalue (`|SpawnActorFromClass` buff (`KismetMathLibrary.MakeTransform` (0.0 0.0 0.0)) "Undefined" "OverrideRootScale" null affectedCharacter turnDuration false false null null))
  (bind (_alreadygotbuff _existingbuff) (`/Game/TurnBasedStrategyRPGTemplate/Blueprints/Units/Characters/BP_CharacterBase.alreadyGotBuff` affectedCharacter _returnvalue))
  (if (not _alreadygotbuff)
    (`/Game/TurnBasedStrategyRPGTemplate/Blueprints/Units/Characters/BP_CharacterBase.AddBuff` affectedCharacter _returnvalue :!label _label)
    (`/Game/TurnBasedStrategyRPGTemplate/Blueprints/StatusEffects/BP_StatusEffectBase.Initialize` _returnvalue)
    (elif (<= (`/Game/TurnBasedStrategyRPGTemplate/Blueprints/StatusEffects/BP_StatusEffectBase.turnDuration` _returnvalue) (`/Game/TurnBasedStrategyRPGTemplate/Blueprints/StatusEffects/BP_StatusEffectBase.turnDuration` _existingbuff))
      (`self.K2_DestroyActor` _returnvalue)
      (else
        (`/Game/TurnBasedStrategyRPGTemplate/Blueprints/StatusEffects/BP_StatusEffectBase.RemoveStatusEffect` _existingbuff)
        (goto _label)))))

(event `AddDebuff`
  (params (affectedCharacter :type "/Game/TurnBasedStrategyRPGTemplate/Blueprints/Units/Characters/BP_CharacterBase Object Reference") (debuff :type "/Game/TurnBasedStrategyRPGTemplate/Blueprints/StatusEffects/Debuffs/BP_DebuffBase Class Reference") (turnDuration :type Integer))
  ;[1 1 1] Add buff / debuff
  (bind _returnvalue (`|SpawnActorFromClass` debuff (`KismetMathLibrary.MakeTransform` (0.0 0.0 0.0)) "Undefined" "OverrideRootScale" null affectedCharacter turnDuration false false null null))
  (bind (_alreadygotdebuff _existingdebuff) (`/Game/TurnBasedStrategyRPGTemplate/Blueprints/Units/Characters/BP_CharacterBase.AlreadyGotDebuff` affectedCharacter _returnvalue))
  (if (not _alreadygotdebuff)
    (`/Game/TurnBasedStrategyRPGTemplate/Blueprints/Units/Characters/BP_CharacterBase.AddDebuff` affectedCharacter _returnvalue :!label _label_2)
    (`/Game/TurnBasedStrategyRPGTemplate/Blueprints/StatusEffects/BP_StatusEffectBase.Initialize` _returnvalue)
    (elif (<= (`/Game/TurnBasedStrategyRPGTemplate/Blueprints/StatusEffects/BP_StatusEffectBase.turnDuration` _returnvalue) (`/Game/TurnBasedStrategyRPGTemplate/Blueprints/StatusEffects/BP_StatusEffectBase.turnDuration` _existingdebuff))
      (`self.K2_DestroyActor` _returnvalue)
      (else
        (`/Game/TurnBasedStrategyRPGTemplate/Blueprints/StatusEffects/BP_StatusEffectBase.RemoveStatusEffect` _existingdebuff)
        (goto _label_2)))))

(event `DamageTargets`
  (params (damageData :type "Map of /Game/TurnBasedStrategyRPGTemplate/Blueprints/Units/Characters/BP_CharacterBase Object Reference to /Game/TurnBasedStrategyRPGTemplate/Blueprints/Structs/S_DamageData Structure"))
  (bind _elementdamagedata (`/Game/TurnBasedStrategyRPGTemplate/Blueprints/Core/BP_BattleController.GetElementReduction` (`self.battleController`) (`self.element`) damageData))
  ;[1 1 1] Damage targets using spell
  (bind _keys (`BlueprintMapLibrary.Map_Keys` _elementdamagedata))
  (for _array_element _keys
    (bind (_damage _mindamage _maxdamage _damagemodifier _element) (break `/Game/TurnBasedStrategyRPGTemplate/Blueprints/Structs/S_DamageData` (`BlueprintMapLibrary.Map_Find` _elementdamagedata _array_element)))
    (`/Game/TurnBasedStrategyRPGTemplate/Blueprints/Units/Characters/BP_CharacterBase.TakeDamage` _array_element _damage _element)))

(event `EndSpell`
  ;[1 1 1] End spell
  (if (`self.animationHasEnded`)
    (`KismetSystemLibrary.RetriggerableDelay` 2.0)
    (`self.OnSpellUseEnded`)
    (else
      (set `self.spellUsed` true))))

(event `SetTargetSlot`
  (params (slot :type "/Game/TurnBasedStrategyRPGTemplate/Blueprints/Grid/Slots/BP_SlotBase Object Reference"))
  ;[1 1 1] Override in child blueprints
)

(fn `GetSpellDamage`
  (params (targetCharacters :type "Array of /Game/TurnBasedStrategyRPGTemplate/Blueprints/Units/Characters/BP_CharacterBase Object Reference"))
  (returns (damageData :type "Map of /Game/TurnBasedStrategyRPGTemplate/Blueprints/Units/Characters/BP_CharacterBase Object Reference to /Game/TurnBasedStrategyRPGTemplate/Blueprints/Structs/S_DamageData Structure"))
  ;[1 1 1] Return damage for the spell
  (return))

(fn `GetSpellSlots`
  (returns (slotsInRange :type "Array of /Game/TurnBasedStrategyRPGTemplate/Blueprints/Grid/Slots/BP_SlotBase Object Reference") (emptySlots :type "Array of /Game/TurnBasedStrategyRPGTemplate/Blueprints/Grid/Slots/BP_SlotBase Object Reference") (allies :type "Array of /Game/TurnBasedStrategyRPGTemplate/Blueprints/Units/Characters/BP_CharacterBase Object Reference") (enemies :type "Array of /Game/TurnBasedStrategyRPGTemplate/Blueprints/Units/Characters/BP_CharacterBase Object Reference"))
  (locals (currentEmptySlots :type "Array of /Game/TurnBasedStrategyRPGTemplate/Blueprints/Grid/Slots/BP_SlotBase Object Reference"))
  (bind _battlecontroller (`self.battleController`))
  ;[1 1 1] Return allies, enemies and empty slots
  (bind _values (`BlueprintMapLibrary.Map_Values` (`/Game/TurnBasedStrategyRPGTemplate/Blueprints/Grid/BP_Grid.slots` (`/Game/TurnBasedStrategyRPGTemplate/Blueprints/Core/BP_BattleController.grid` (`self.battleController`)))))
  (for _array_element _values
    (if (`/Game/TurnBasedStrategyRPGTemplate/Blueprints/Grid/Slots/BP_SlotBase.IsEmpty` _array_element)
      (`KismetArrayLibrary.Array_Add` (`local.currentEmptySlots`) _array_element)))
  (return _values (`local.currentEmptySlots`) (`/Game/TurnBasedStrategyRPGTemplate/Blueprints/Core/BP_BattleController.playerCharacters` _battlecontroller) (`/Game/TurnBasedStrategyRPGTemplate/Blueprints/Core/BP_BattleController.enemyCharacters` _battlecontroller)))

(fn `UserConstructionScript`)