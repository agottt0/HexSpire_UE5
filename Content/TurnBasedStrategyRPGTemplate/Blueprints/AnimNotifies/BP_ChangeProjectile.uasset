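; Anim notify state that temporarily swaps the projectile of a ranged character during an animation.
; On begin, it casts the mesh owner to BP_RangeCharacterBase and passes its Projectile variable to ChangeProjectile.
; On end, it calls ResetProjectile on the same character to restore it.
; Both events return false when the owner is not a ranged character.
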(fn `Received_NotifyBegin`
  (params (MeshComp :type "SkeletalMeshComponent Object Reference") (Animation :type "AnimSequenceBase Object Reference") (TotalDuration :type "Float (double-precision)"))
  (returns (ReturnValue :type Boolean))
  ;[1 1 1] Change projectile
  (bind _asbp_range_character_base (cast `/Game/TurnBasedStrategyRPGTemplate/Blueprints/Units/Characters/RangeCharacters/BP_RangeCharacterBase` (`ActorComponent.GetOwner` MeshComp))
    (:`then`
      (`/Game/TurnBasedStrategyRPGTemplate/Blueprints/Units/Characters/RangeCharacters/BP_RangeCharacterBase.ChangeProjectile` _asbp_range_character_base (`self.projectile`))
      (return true))
    (:`CastFailed`
      (return false))))

(fn `Received_NotifyEnd`
  (params (MeshComp :type "SkeletalMeshComponent Object Reference") (Animation :type "AnimSequenceBase Object Reference"))
  (returns (ReturnValue :type Boolean))
  ;[1 1 1] Reset projectile
  (bind _asbp_range_character_base (cast `/Game/TurnBasedStrategyRPGTemplate/Blueprints/Units/Characters/RangeCharacters/BP_RangeCharacterBase` (`ActorComponent.GetOwner` MeshComp))
    (:`then`
      (`/Game/TurnBasedStrategyRPGTemplate/Blueprints/Units/Characters/RangeCharacters/BP_RangeCharacterBase.ResetProjectile` _asbp_range_character_base)
      (return true))
    (:`CastFailed`
      (return false))))