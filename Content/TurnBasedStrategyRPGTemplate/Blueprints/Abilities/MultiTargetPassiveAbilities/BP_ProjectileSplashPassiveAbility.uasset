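; Passive multi-target ability for projectile splash damage, selecting the enemies around an attacked slot in the turn-based grid combat.
; GetEnemiesInAbilityRange asks the BattleController's grid for all slots, occupied or empty, within Range of the attack slot, ignoring the standing slot.
; It returns each unique character in those slots that is an enemy of the ability owner.
; This Blueprint only gathers targets and applies no damage itself.
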(fn `GetEnemiesInAbilityRange`
  (params (attackSlot :type "/Game/TurnBasedStrategyRPGTemplate/Blueprints/Grid/Slots/BP_SlotBase Object Reference") (standingSlot :type "/Game/TurnBasedStrategyRPGTemplate/Blueprints/Grid/Slots/BP_SlotBase Object Reference"))
  (returns (enemies :type "Array of /Game/TurnBasedStrategyRPGTemplate/Blueprints/Units/Characters/BP_CharacterBase Object Reference"))
  ;[1 1 1] Return enemies around targeted slot
  ; Range 1 = targeted slot
  ; Range 3 = targeted slot and its neighbours
  (`KismetArrayLibrary.Array_Clear` (`self.enemyCharacters`))
  (bind _slotsinrange (`/Game/TurnBasedStrategyRPGTemplate/Blueprints/Grid/BP_Grid.GetSlotsInRange` (`/Game/TurnBasedStrategyRPGTemplate/Blueprints/Core/BP_BattleController.grid` (`self.battleController`)) attackSlot (`self.range`) false))
  (for _array_element _slotsinrange
    (bind (_isenemyslot _enemycharacter) (`/Game/TurnBasedStrategyRPGTemplate/Blueprints/Grid/Slots/BP_SlotBase.IsEnemySlot` _array_element (`self.abilityOwner`)))
    (if _isenemyslot
      (`KismetArrayLibrary.Array_AddUnique` (`self.enemyCharacters`) _enemycharacter)))
  (return (`self.enemyCharacters`)))

(fn `UserConstructionScript`
  (`parent.UserConstructionScript`))