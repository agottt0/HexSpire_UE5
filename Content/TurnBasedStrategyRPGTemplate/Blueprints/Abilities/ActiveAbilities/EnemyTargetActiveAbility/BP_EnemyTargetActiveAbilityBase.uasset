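; Base active ability that targets enemies in the turn-based battle system, available only when its melee/ranged type matches the attack and enemy slots exist.
; While enabled, it can spawn a multi-target ability that temporarily replaces the owner's passive one, restoring the default when disabled.
; Playing the animation sets cooldown and spends mana.
; Status effects route through OnAbilityUsed, timed before or after the attack by RemoveStatusEffectAfterAttack.
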(event `self.OnActiveAbilityEnabled`
  ;[1 1 1] Replace multi target ability from the active ability with the default one
  (if (`KismetSystemLibrary.IsValidClass` (`self.multiTargetAbility`))
    (set `self.defaultMultiTargetAbility` (`/Game/TurnBasedStrategyRPGTemplate/Blueprints/Units/Characters/BP_CharacterBase.currentMultiTargetPassiveAbility` (`self.abilityOwner`)))
    (bind _returnvalue (`|SpawnActorFromClass` (`self.multiTargetAbility`) (`KismetMathLibrary.MakeTransform` (0.0 0.0 0.0)) "Undefined" "OverrideRootScale" null (`self.abilityOwner`) (`self.battleController`) null))
    (bind _output_get (set `self.currentMultiTargetAbility` _returnvalue))
    (set `/Game/TurnBasedStrategyRPGTemplate/Blueprints/Units/Characters/BP_CharacterBase.currentMultiTargetPassiveAbility` _output_get (`self.abilityOwner`))))

(event `self.OnActiveAbilityDisabled`
  ;[1 1 1] Replace multi target ability from the active ability with the default one
  (if (`KismetSystemLibrary.IsValidClass` (`self.multiTargetAbility`))
    (`self.K2_DestroyActor` (`self.currentMultiTargetAbility`))
    (set `/Game/TurnBasedStrategyRPGTemplate/Blueprints/Units/Characters/BP_CharacterBase.currentMultiTargetPassiveAbility` (`self.defaultMultiTargetAbility`) (`self.abilityOwner`))))

(event `self.PlayAbilityAnimation`
  ;[1 1 1] Set cooldown
  (`self.SetCooldown` (+ (`self.cooldown`) 1))
  (`self.ReduceMana`))

(event `self.ApplyStatusEffects`
  (params (allyCharacters :type "Array of /Game/TurnBasedStrategyRPGTemplate/Blueprints/Units/Characters/BP_CharacterBase Object Reference (by ref)") (enemyCharacters :type "Array of /Game/TurnBasedStrategyRPGTemplate/Blueprints/Units/Characters/BP_CharacterBase Object Reference (by ref)") (isBeforeAttack :type Boolean))
  (bind _array (`|MakeArray` null :!type "/Game/TurnBasedStrategyRPGTemplate/Blueprints/Grid/Slots/BP_SlotBase Object Reference"))
  ;[1 1 1] Add status effects for the ability
  (if (== isBeforeAttack (`self.removeStatusEffectAfterAttack`))
    (`self.OnAbilityUsed` _array _array allyCharacters enemyCharacters)))

(fn `IsAvailable`
  (params (isMeleeAttack :type Boolean))
  (returns (isAvailable :type Boolean))
  ;[1 1 1] Checks if character and ability are both melee or both range and has enemy in range
  (bind _isavailable (`parent.IsAvailable` isMeleeAttack))
  (return (and _isavailable (== isMeleeAttack (`self.isMelee`)) (> (`KismetArrayLibrary.Array_Length` (`/Game/TurnBasedStrategyRPGTemplate/Blueprints/Grid/BP_Grid.enemySlots` (`/Game/TurnBasedStrategyRPGTemplate/Blueprints/Core/BP_BattleController.grid` (`self.battleController`)))) 0))))

(fn `UserConstructionScript`
  (`parent.UserConstructionScript`))