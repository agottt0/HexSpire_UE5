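; Greater Heal, an instant-cast active ability for the turn-based strategy RPG that heals every ally in range.
; On use it applies a fixed heal to each ally passed in, then ends the turn.
; Its AI usage check returns true when at least one ally in range is missing a set amount of health.
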(event `self.OnAbilityUsed`
  (params (slotsInRange :type "Array of /Game/TurnBasedStrategyRPGTemplate/Blueprints/Grid/Slots/BP_SlotBase Object Reference (by ref)") (emptySlotsInRange :type "Array of /Game/TurnBasedStrategyRPGTemplate/Blueprints/Grid/Slots/BP_SlotBase Object Reference (by ref)") (alliesInRange :type "Array of /Game/TurnBasedStrategyRPGTemplate/Blueprints/Units/Characters/BP_CharacterBase Object Reference (by ref)") (enemiesInRange :type "Array of /Game/TurnBasedStrategyRPGTemplate/Blueprints/Units/Characters/BP_CharacterBase Object Reference (by ref)"))
  ;[1 1 1] Heals allies 50 points in range
  (for _array_element alliesInRange
    (`/Game/TurnBasedStrategyRPGTemplate/Blueprints/Units/Characters/BP_CharacterBase.Heal` _array_element 50))
  (`self.EndTurn`))

(fn `ShouldAIUse`
  (params (slotsInRange :type "Array of /Game/TurnBasedStrategyRPGTemplate/Blueprints/Grid/Slots/BP_SlotBase Object Reference (by ref)") (emptySlotsInRange :type "Array of /Game/TurnBasedStrategyRPGTemplate/Blueprints/Grid/Slots/BP_SlotBase Object Reference (by ref)") (alliesInRange :type "Array of /Game/TurnBasedStrategyRPGTemplate/Blueprints/Units/Characters/BP_CharacterBase Object Reference (by ref)") (enemiesInRange :type "Array of /Game/TurnBasedStrategyRPGTemplate/Blueprints/Units/Characters/BP_CharacterBase Object Reference (by ref)") (weakestEnemy :type "/Game/TurnBasedStrategyRPGTemplate/Blueprints/Units/Characters/BP_CharacterBase Object Reference"))
  (returns (shouldAIUse :type Boolean))
  (locals (currentShouldAIUse :type Boolean :default false))
  ;[1 1 1] AI uses this ability when there is an ally character around it that lost 25 health points
  (for _array_element alliesInRange
    (bind _characterstats_maxhealth (break `/Game/TurnBasedStrategyRPGTemplate/Blueprints/Structs/S_CharacterStats` (`/Game/TurnBasedStrategyRPGTemplate/Blueprints/Units/Characters/BP_CharacterBase.characterStats` _array_element)))
    (if (>= (- _characterstats_maxhealth (`/Game/TurnBasedStrategyRPGTemplate/Blueprints/Units/Characters/BP_CharacterBase.currentHealth` _array_element)) 25)
      (set `local.currentShouldAIUse` true)))
  (return (`local.currentShouldAIUse`)))

(fn `UserConstructionScript`
  (`parent.UserConstructionScript`))