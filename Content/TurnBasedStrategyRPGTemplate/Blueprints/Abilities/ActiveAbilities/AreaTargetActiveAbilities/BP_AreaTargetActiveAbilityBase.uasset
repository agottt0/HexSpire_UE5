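; Base Blueprint for area-target active abilities in a turn-based strategy RPG, affecting slots around a chosen target slot.
; Enabling or disabling the ability notifies the battle grid, which works with the stored target slot.
; GetAbilitySlots sorts slots within range of that target into empty slots, allies and enemies.
; AI targets a random ally, enemy or any slot based on highlight flags, and uses the ability whenever a target is set.
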(event `self.OnActiveAbilityEnabled`
  ;[1 1 1] Enable / disable area target ability
  (`/Game/TurnBasedStrategyRPGTemplate/Blueprints/Grid/BP_Grid.OnAreaTargetAbilityEnabled` (`/Game/TurnBasedStrategyRPGTemplate/Blueprints/Core/BP_BattleController.grid` (`self.battleController`)) self))

(event `self.OnActiveAbilityDisabled`
  ;[1 1 1] Enable / disable area target ability
  (`/Game/TurnBasedStrategyRPGTemplate/Blueprints/Grid/BP_Grid.OnAreaTargetAbilityDisabled` (`/Game/TurnBasedStrategyRPGTemplate/Blueprints/Core/BP_BattleController.grid` (`self.battleController`))))

(event `self.ResetTargetSlot`
  ;[1 1 1] Reset target slot
  (`self.SetTargetSlot` null))

(event `self.SetTargetSlot`
  (params (slot :type "/Game/TurnBasedStrategyRPGTemplate/Blueprints/Grid/Slots/BP_SlotBase Object Reference"))
  ;[1 1 1] Set target slot for the ability
  (set `self.targetSlot` slot))

(event `self.SetTargetSlotForAI`
  ;[1 1 1] Set target slot for enemy
  (if (`self.highlightAllies`)
    (set `self.targetSlot` (`/Game/TurnBasedStrategyRPGTemplate/Blueprints/Units/BP_UnitBase.slot` (`KismetArrayLibrary.Array_Random` (select `bool` (`/Game/TurnBasedStrategyRPGTemplate/Blueprints/Units/Characters/BP_CharacterBase.isAI` (`self.abilityOwner`)) :`false` (`/Game/TurnBasedStrategyRPGTemplate/Blueprints/Core/BP_BattleController.playerCharacters` (`self.battleController`)) :`true` (`/Game/TurnBasedStrategyRPGTemplate/Blueprints/Core/BP_BattleController.enemyCharacters` (`self.battleController`))))))
    (elif (`self.highlightEnemies`)
      (set `self.targetSlot` (`/Game/TurnBasedStrategyRPGTemplate/Blueprints/Units/BP_UnitBase.slot` (`KismetArrayLibrary.Array_Random` (select `bool` (`/Game/TurnBasedStrategyRPGTemplate/Blueprints/Units/Characters/BP_CharacterBase.isAI` (`self.abilityOwner`)) :`false` (`/Game/TurnBasedStrategyRPGTemplate/Blueprints/Core/BP_BattleController.enemyCharacters` (`self.battleController`)) :`true` (`/Game/TurnBasedStrategyRPGTemplate/Blueprints/Core/BP_BattleController.playerCharacters` (`self.battleController`))))))
      (else
        (bind _values (`BlueprintMapLibrary.Map_Values` (`/Game/TurnBasedStrategyRPGTemplate/Blueprints/Grid/BP_Grid.slots` (`/Game/TurnBasedStrategyRPGTemplate/Blueprints/Core/BP_BattleController.grid` (`self.battleController`)))))
        (set `self.targetSlot` (`KismetArrayLibrary.Array_Random` _values))))))

(fn `GetAbilityDamage`
  (params (targetCharacters :type "Array of /Game/TurnBasedStrategyRPGTemplate/Blueprints/Units/Characters/BP_CharacterBase Object Reference"))
  (returns (damageData :type "Map of /Game/TurnBasedStrategyRPGTemplate/Blueprints/Units/Characters/BP_CharacterBase Object Reference to /Game/TurnBasedStrategyRPGTemplate/Blueprints/Structs/S_DamageData Structure"))
  ;[1 1 1] Return damage for the ability
  (return))

(fn `GetAbilitySlots`
  (returns (slotsInRange :type "Array of /Game/TurnBasedStrategyRPGTemplate/Blueprints/Grid/Slots/BP_SlotBase Object Reference") (emptySlotsInRange :type "Array of /Game/TurnBasedStrategyRPGTemplate/Blueprints/Grid/Slots/BP_SlotBase Object Reference") (alliesInRange :type "Array of /Game/TurnBasedStrategyRPGTemplate/Blueprints/Units/Characters/BP_CharacterBase Object Reference") (enemiesInRange :type "Array of /Game/TurnBasedStrategyRPGTemplate/Blueprints/Units/Characters/BP_CharacterBase Object Reference"))
  (locals (currentEnemies :type "Array of /Game/TurnBasedStrategyRPGTemplate/Blueprints/Units/Characters/BP_CharacterBase Object Reference") (currentAllies :type "Array of /Game/TurnBasedStrategyRPGTemplate/Blueprints/Units/Characters/BP_CharacterBase Object Reference") (emptySlots :type "Array of /Game/TurnBasedStrategyRPGTemplate/Blueprints/Grid/Slots/BP_SlotBase Object Reference"))
  ;[1 1 1] Return all slots, empty slots, enemies and allies in range
  (`/Engine/EditorBlueprintResources/StandardMacros.IsValid` (`self.targetSlot`)
    (:`Is Valid`
      (bind _slotsinrange (`/Game/TurnBasedStrategyRPGTemplate/Blueprints/Grid/BP_Grid.GetSlotsInRange` (`/Game/TurnBasedStrategyRPGTemplate/Blueprints/Core/BP_BattleController.grid` (`self.battleController`)) (`self.targetSlot`) (`self.range`) false))
      (for _array_element _slotsinrange
        (if (`/Game/TurnBasedStrategyRPGTemplate/Blueprints/Grid/Slots/BP_SlotBase.IsEmpty` _array_element)
          (`KismetArrayLibrary.Array_AddUnique` (`local.emptySlots`) _array_element)
          (else
            (bind (_isenemyslot _enemycharacter) (`/Game/TurnBasedStrategyRPGTemplate/Blueprints/Grid/Slots/BP_SlotBase.IsEnemySlot` _array_element (`self.abilityOwner`)))
            (if _isenemyslot
              (`KismetArrayLibrary.Array_AddUnique` (`local.currentEnemies`) _enemycharacter)
              (else
                (bind (_isallyslot _allycharacter) (`/Game/TurnBasedStrategyRPGTemplate/Blueprints/Grid/Slots/BP_SlotBase.IsAllySlot` _array_element (`self.abilityOwner`)))
                (if _isallyslot
                  (`KismetArrayLibrary.Array_AddUnique` (`local.currentAllies`) _allycharacter))))))))
    (:`Is Not Valid`
      _))
  (return _slotsinrange (`local.emptySlots`) (`local.currentAllies`) (`local.currentEnemies`)))

(fn `ShouldAIUse`
  (params (slotsInRange :type "Array of /Game/TurnBasedStrategyRPGTemplate/Blueprints/Grid/Slots/BP_SlotBase Object Reference (by ref)") (emptySlotsInRange :type "Array of /Game/TurnBasedStrategyRPGTemplate/Blueprints/Grid/Slots/BP_SlotBase Object Reference (by ref)") (alliesInRange :type "Array of /Game/TurnBasedStrategyRPGTemplate/Blueprints/Units/Characters/BP_CharacterBase Object Reference (by ref)") (enemiesInRange :type "Array of /Game/TurnBasedStrategyRPGTemplate/Blueprints/Units/Characters/BP_CharacterBase Object Reference (by ref)") (weakestEnemy :type "/Game/TurnBasedStrategyRPGTemplate/Blueprints/Units/Characters/BP_CharacterBase Object Reference"))
  (returns (shouldAIUse :type Boolean))
  ;[1 1 1] AI uses if target slot is set
  (`/Engine/EditorBlueprintResources/StandardMacros.IsValid` (`self.targetSlot`)
    (:`Is Valid`
      (return true))
    (:`Is Not Valid`
      (return false))))

(fn `UserConstructionScript`
  (`parent.UserConstructionScript`))