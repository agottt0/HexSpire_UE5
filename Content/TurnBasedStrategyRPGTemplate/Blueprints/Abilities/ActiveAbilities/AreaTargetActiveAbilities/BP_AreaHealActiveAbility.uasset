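; Area-target active ability for the turn-based RPG template that heals allies within range.
; On use, it heals each ally in range by a fixed amount and then ends the turn.
; For AI targeting, it picks the slot of the first character on the owner's side missing at least that amount of health.
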(event `self.OnAbilityUsed`
  (params (slotsInRange :type "Array of /Game/TurnBasedStrategyRPGTemplate/Blueprints/Grid/Slots/BP_SlotBase Object Reference (by ref)") (emptySlotsInRange :type "Array of /Game/TurnBasedStrategyRPGTemplate/Blueprints/Grid/Slots/BP_SlotBase Object Reference (by ref)") (alliesInRange :type "Array of /Game/TurnBasedStrategyRPGTemplate/Blueprints/Units/Characters/BP_CharacterBase Object Reference (by ref)") (enemiesInRange :type "Array of /Game/TurnBasedStrategyRPGTemplate/Blueprints/Units/Characters/BP_CharacterBase Object Reference (by ref)"))
  ;[1 1 1] Heal allies in range
  (for _array_element alliesInRange
    (`/Game/TurnBasedStrategyRPGTemplate/Blueprints/Units/Characters/BP_CharacterBase.Heal` _array_element 25))
  (`self.EndTurn`))

(event `self.SetTargetSlotForAI`
  ;[1 1 1] AI finds an ally character that lost 25 health points
  (for _array_element (select `bool` (`/Game/TurnBasedStrategyRPGTemplate/Blueprints/Units/Characters/BP_CharacterBase.isAI` (`self.abilityOwner`)) :`false` (`/Game/TurnBasedStrategyRPGTemplate/Blueprints/Core/BP_BattleController.playerCharacters` (`self.battleController`)) :`true` (`/Game/TurnBasedStrategyRPGTemplate/Blueprints/Core/BP_BattleController.enemyCharacters` (`self.battleController`)))
    (bind _mainstats_maxhealth (break `/Game/TurnBasedStrategyRPGTemplate/Blueprints/Structs/S_CharacterStats` (`/Game/TurnBasedStrategyRPGTemplate/Blueprints/Units/Characters/BP_CharacterBase.mainStats` _array_element)))
    (if (>= (- _mainstats_maxhealth (`/Game/TurnBasedStrategyRPGTemplate/Blueprints/Units/Characters/BP_CharacterBase.currentHealth` _array_element)) 25)
      (`self.SetTargetSlot` (`/Game/TurnBasedStrategyRPGTemplate/Blueprints/Units/BP_UnitBase.slot` _array_element))
      (break))))

(fn `UserConstructionScript`
  (`parent.UserConstructionScript`))