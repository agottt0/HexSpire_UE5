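; Base quest Blueprint for battle quests, where each entry in the EnemyPawn array is one step.
; At start it deactivates all those pawns; activating a step enables that pawn's interaction detector, found through its ChildActorComponent.
; With HideActors set, inactive pawns are also disabled, while activation restores the current and earlier ones and completion restores all.
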(event `self.ReceiveBeginPlay`
  ;[1 1 1] Disable quest actors at start
  (for _array_element (`self.enemyPawn`)
    (`self.SetQuestActors` _array_element)))

(event `SetQuestActors`
  (params (actor :type "Actor Object Reference") (isActive :type Boolean))
  (bind _returnvalue (`self.GetComponentByClass` actor "/Script/Engine.ChildActorComponent"))
  ;[1 1 1] Disable interactables at start
  (`/Engine/EditorBlueprintResources/StandardMacros.IsValid` actor
    (:`Is Valid`
      (if (`self.hideActors`)
        (`/Game/TurnBasedStrategyRPGTemplate/Blueprints/Core/BP_RPGFunctionLibrary.DisableActor` actor (not isActive)))
      (`/Engine/EditorBlueprintResources/StandardMacros.IsValid` _returnvalue
        (:`Is Valid`
          (bind _asbp_interaction_detector (cast `/Game/TurnBasedStrategyRPGTemplate/Blueprints/Interactables/BP_InteractionDetector` (`ChildActorComponent.ChildActor` _returnvalue)))
          (if isActive
            (`/Game/TurnBasedStrategyRPGTemplate/Blueprints/Interactables/BP_InteractionDetector.EnableInteraction` _asbp_interaction_detector)
            (else
              (`/Game/TurnBasedStrategyRPGTemplate/Blueprints/Interactables/BP_InteractionDetector.DisableInteraction` _asbp_interaction_detector))))))))

(event `self.Activate`
  (params (currentStep :type Integer))
  ;[1 1 1] Activate quest actors
  (`self.SetQuestActors` (`|GetArrayItem` (`self.enemyPawn`) currentStep) true)
  (if (`self.hideActors`)
    (for (_array_element _array_index) (`self.enemyPawn`)
      (`/Engine/EditorBlueprintResources/StandardMacros.IsValid` _array_element
        (:`Is Valid`
          (if (< _array_index currentStep)
            (`/Game/TurnBasedStrategyRPGTemplate/Blueprints/Core/BP_RPGFunctionLibrary.DisableActor` _array_element)))))))

(event `self.Completed`
  ;[1 1 1] Enable quest actors after completed
  (if (`self.hideActors`)
    (for _array_element (`self.enemyPawn`)
      (`/Engine/EditorBlueprintResources/StandardMacros.IsValid` _array_element
        (:`Is Valid`
          (`/Game/TurnBasedStrategyRPGTemplate/Blueprints/Core/BP_RPGFunctionLibrary.DisableActor` _array_element))))))

(fn `GetSteps`
  (returns (steps :type Integer))
  ;[1 1 1] Return number of steps to completed this quest
  (return (`KismetArrayLibrary.Array_Length` (`self.enemyPawn`))))

(fn `UserConstructionScript`
  (`parent.UserConstructionScript`))