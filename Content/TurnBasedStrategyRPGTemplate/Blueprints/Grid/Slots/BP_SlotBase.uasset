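; Base grid slot for turn-based combat, tracking its contained unit, pathfinding data, attack-from slots and auras.
; Slot type drives the Paper2D sprite and opacity, choosing from per-unit-size sprite sets, with a saved previous type restored when highlighting ends.
; Ally and enemy checks compare IsAI on living characters, deciding whether auras apply buffs or debuffs to the occupant.
; Auras clear through their owner's removed-from-slot callback; children override ClearAllCallbacks.
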(event `Initialize`
  (params (slotSize :type "Vector Structure") (slotSpriteSize :type "Vector Structure") (`1x1SlotSprites` :type "/Game/TurnBasedStrategyRPGTemplate/Blueprints/Structs/S_SlotSprites Structure") (`2x2SlotSprites` :type "/Game/TurnBasedStrategyRPGTemplate/Blueprints/Structs/S_SlotSprites Structure") (`3x3SlotSprites` :type "/Game/TurnBasedStrategyRPGTemplate/Blueprints/Structs/S_SlotSprites Structure") (`4x4SlotSprites` :type "/Game/TurnBasedStrategyRPGTemplate/Blueprints/Structs/S_SlotSprites Structure") (`5x5SlotSprites` :type "/Game/TurnBasedStrategyRPGTemplate/Blueprints/Structs/S_SlotSprites Structure") (`6x6SlotSprites` :type "/Game/TurnBasedStrategyRPGTemplate/Blueprints/Structs/S_SlotSprites Structure") (`7x7SlotSprites` :type "/Game/TurnBasedStrategyRPGTemplate/Blueprints/Structs/S_SlotSprites Structure") (`8x8SlotSprites` :type "/Game/TurnBasedStrategyRPGTemplate/Blueprints/Structs/S_SlotSprites Structure"))
  ;[1 1 1] Initialize
  (set `self.slotSize` slotSize)
  (bind _output_get (set `self.slotSpriteSize` slotSpriteSize))
  (`SceneComponent.SetWorldScale3D` (`self.PaperSprite`) _output_get)
  (set `self.1x1SlotSprites` `1x1SlotSprites`)
  (set `self.2x2SlotSprites` `2x2SlotSprites`)
  (set `self.3x3SlotSprites` `3x3SlotSprites`)
  (set `self.4x4SlotSprites` `4x4SlotSprites`)
  (set `self.5x5SlotSprites` `5x5SlotSprites`)
  (set `self.6x6SlotSprites` `6x6SlotSprites`)
  (set `self.7x7SlotSprites` `7x7SlotSprites`)
  (set `self.8x8SlotSprites` `8x8SlotSprites`))

(event `SetUnit`
  (params (unit :type "/Game/TurnBasedStrategyRPGTemplate/Blueprints/Units/BP_UnitBase Object Reference"))
  ;[1 1 1] Set contained unit
  (set `self.containedUnit` unit))

(event `SetSlotType`
  (params (slotType :type "/Game/TurnBasedStrategyRPGTemplate/Blueprints/Enums/E_SlotType Enum" :default "NewEnumerator0") (size :type Integer :default 1))
  (bind (_slotspritestruct_defaultslotsprite _slotspritestruct_movableslotsprite _slotspritestruct_activeslotsprite _slotspritestruct_enemyslotsprite _slotspritestruct_allyslotsprite _slotspritestruct_movementoverlayslotsprite _slotspritestruct_spellslotsprite) (break `/Game/TurnBasedStrategyRPGTemplate/Blueprints/Structs/S_SlotSprites` (`self.GetSlotSpriteStruct` size)))
  (bind _slottype (`self.slotType`))
  ;[1 1 1] Slot sprite logic
  (set `self.slotType` slotType)
  (`PaperSpriteComponent.SetSprite` (`self.PaperSprite`) (select `/Game/TurnBasedStrategyRPGTemplate/Blueprints/Enums/E_SlotType` _slottype :`NewEnumerator1` _slotspritestruct_defaultslotsprite :`NewEnumerator2` _slotspritestruct_movableslotsprite :`NewEnumerator3` _slotspritestruct_activeslotsprite :`NewEnumerator4` _slotspritestruct_enemyslotsprite :`NewEnumerator5` _slotspritestruct_allyslotsprite :`NewEnumerator6` _slotspritestruct_movementoverlayslotsprite :`NewEnumerator7` _slotspritestruct_spellslotsprite))
  (`PaperSpriteComponent.SetSpriteColor` (`self.PaperSprite`) (make `LinearColor` 1.0 1.0 1.0 (select `/Game/TurnBasedStrategyRPGTemplate/Blueprints/Enums/E_SlotType` _slottype :`NewEnumerator0` 1.0 :`NewEnumerator1` 0.1 :`NewEnumerator2` 0.5 :`NewEnumerator3` 1.0 :`NewEnumerator4` 1.0 :`NewEnumerator5` 1.0 :`NewEnumerator6` 1.0 :`NewEnumerator7` 1.0 :!type "Float (single-precision)"))))

(event `SaveSlotType`
  ;[1 1 1] Slot sprite logic
  (set `self.previousSlotType` (`self.slotType`)))

(event `HideSlot`
  ;[1 1 1] Slot sprite logic
  (`self.SetSlotType` "NewEnumerator0"))

(event `SetSpellSlot`
  ;[1 1 1] Slot sprite logic
  (`self.SetSlotType` "NewEnumerator7"))

(event `Movable`
  (params (isOn :type Boolean))
  ;[1 1 1] Slot sprite logic
  (bind _output_get (set `self.isMovable` isOn))
  (`self.SetSlotType` (select `bool` _output_get :`false` "NewEnumerator1" :`true` "NewEnumerator2" :!type "/Game/TurnBasedStrategyRPGTemplate/Blueprints/Enums/E_SlotType Enum")))

(event `SetEnemySlot`
  (params (size :type Integer))
  ;[1 1 1] Slot sprite logic
  (`self.SetSlotType` "NewEnumerator4" size))

(event `SetAllySlot`
  (params (size :type Integer))
  ;[1 1 1] Slot sprite logic
  (`self.SetSlotType` "NewEnumerator5" size))

(event `Highlight`
  (params (isOn :type Boolean) (size :type Integer :default 1))
  ;[1 1 1] Slot sprite logic
  (if isOn
    (`self.SetSlotType` "NewEnumerator3" size)
    (else
      (`self.SetSlotType` (`self.previousSlotType`)))))

(event `SetPlayerSpawnSlot`
  ;[1 1 1] Set as player spawn slot
  (set `self.canPlayerCharacterSpawn` true)
  (`self.SetSlotType` "NewEnumerator2"))

(event `ShowTotalCost`
  ;[1 1 1] Debug pathfinding
  (`TextRenderComponent.K2_SetText` (`self.TotalCostText`) (`KismetTextLibrary.Conv_IntToText` (`self.totalCost`)))
  (`SceneComponent.SetVisibility` (`self.TotalCostText`) true false))

(event `ResetMovementData`
  (params (isOverlayData :type Boolean))
  ;[1 1 1] Reset pathfinding data
  (set `self.totalCost` 0)
  (set `self.parent` null)
  (`KismetArrayLibrary.Array_Clear` (select `bool` isOverlayData :`false` (`self.path`) :`true` (`self.overlayPath`))))

(event `AddSlotToCanAttackFromSlots`
  (params (slot :type "/Game/TurnBasedStrategyRPGTemplate/Blueprints/Grid/Slots/BP_SlotBase Object Reference"))
  ;[1 1 1] Add / clear attack data
  (`KismetArrayLibrary.Array_AddUnique` (`self.canAttackFromSlots`) slot))

(event `ClearCanAttackFromSlots`
  ;[1 1 1] Add / clear attack data
  (`KismetArrayLibrary.Array_Clear` (`self.canAttackFromSlots`)))

(event `AddAura`
  (params (aura :type "/Game/TurnBasedStrategyRPGTemplate/Blueprints/Abilities/Auras/BP_AuraBase Object Reference") (auraOwner :type "/Game/TurnBasedStrategyRPGTemplate/Blueprints/Units/Characters/BP_CharacterBase Object Reference"))
  ;[1 1 1] Add / remove aura on the slot
  (`BlueprintMapLibrary.Map_Add` (`self.auras`) aura auraOwner)
  (add `/Game/TurnBasedStrategyRPGTemplate/Blueprints/Units/Characters/BP_CharacterBase.OnCharacterRemovedFromSlot` auraOwner (delegate `OnCharacterRemovedFromSlotHandler`)))

(event `OnCharacterRemovedFromSlotHandler`
  (params (character :type "/Game/TurnBasedStrategyRPGTemplate/Blueprints/Units/Characters/BP_CharacterBase Object Reference"))
  ;[1 1 1] Add / remove aura on the slot
  (remove `/Game/TurnBasedStrategyRPGTemplate/Blueprints/Units/Characters/BP_CharacterBase.OnCharacterRemovedFromSlot` character (delegate `OnCharacterRemovedFromSlotHandler`))
  (`self.RemoveAura` character))

(event `RemoveAura`
  (params (auraOwner :type "/Game/TurnBasedStrategyRPGTemplate/Blueprints/Units/Characters/BP_CharacterBase Object Reference"))
  (bind _auras (`self.auras`))
  ;[1 1 1] Add / remove aura on the slot
  (bind _keys (`BlueprintMapLibrary.Map_Keys` _auras))
  (bind (_arrayindex _arrayelement) (`/Engine/EditorBlueprintResources/StandardMacros.ReverseForEachLoop` _keys)
    (:`LoopBody`
      (if (== (`BlueprintMapLibrary.Map_Find` _auras _arrayelement) auraOwner)
        (`BlueprintMapLibrary.Map_Remove` (`self.auras`) _arrayelement)))))

(event `ApplyAuraToContainedUnit`
  (bind _auras (`self.auras`))
  ;[1 1 1] Apply aura to the character that is on the slot
  (bind _keys (`BlueprintMapLibrary.Map_Keys` _auras))
  (bind (_arrayindex _arrayelement) (`/Engine/EditorBlueprintResources/StandardMacros.ReverseForEachLoop` _keys)
    (:`LoopBody`
      (bind _value (`BlueprintMapLibrary.Map_Find` _auras _arrayelement))
      (bind (_isallyslot _allycharacter) (`self.IsAllySlot` _value))
      (if _isallyslot
        (`/Game/TurnBasedStrategyRPGTemplate/Blueprints/Abilities/Auras/BP_AuraBase.AddBuffsToCharacter` _arrayelement _allycharacter)
        (else
          (bind (_isenemyslot _enemycharacter) (`self.IsEnemySlot` _value))
          (if _isenemyslot
            (`/Game/TurnBasedStrategyRPGTemplate/Blueprints/Abilities/Auras/BP_AuraBase.AddDebuffsToCharacter` _arrayelement _enemycharacter)))))))

(event `ClearAllCallbacks`
  ;[1 1 1] Override in children blueprints
)

(fn `ContainsObstacle`
  (returns (containsObstacle :type Boolean))
  ;[1 1 1] Check if the slot contains obstacle
  (return (`.bSuccess` (cast `/Game/TurnBasedStrategyRPGTemplate/Blueprints/Units/Obstacles/BP_ObstacleBase` (`self.containedUnit`) :!pure true))))

(fn `GetSlotSpriteStruct`
  (params (size :type Integer))
  (returns (slotSpriteStruct :type "/Game/TurnBasedStrategyRPGTemplate/Blueprints/Structs/S_SlotSprites Structure"))
  ;[1 1 1] Returns slot sprites based on unit size
  (return (select `int` size :`0` (struct) :`1` (`self.1x1SlotSprites`) :`2` (`self.2x2SlotSprites`) :`3` (`self.3x3SlotSprites`) :`4` (`self.4x4SlotSprites`) :`5` (`self.5x5SlotSprites`) :`6` (`self.6x6SlotSprites`) :`7` (`self.7x7SlotSprites`) :`8` (`self.8x8SlotSprites`))))

(fn `IsAllySlot`
  (params (character :type "/Game/TurnBasedStrategyRPGTemplate/Blueprints/Units/Characters/BP_CharacterBase Object Reference"))
  (returns (isAllySlot :type Boolean) (allyCharacter :type "/Game/TurnBasedStrategyRPGTemplate/Blueprints/Units/Characters/BP_CharacterBase Object Reference"))
  ;[1 1 1] Check if the slot contains enemy unit
  (bind _asbp_character_base (cast `/Game/TurnBasedStrategyRPGTemplate/Blueprints/Units/Characters/BP_CharacterBase` (`self.containedUnit`))
    (:`then`
      (bind _isdead (`/Game/TurnBasedStrategyRPGTemplate/Blueprints/Units/Characters/BP_CharacterBase.IsDead` _asbp_character_base))
      (if _isdead
        (return false null)
        (else
          (return (== (`/Game/TurnBasedStrategyRPGTemplate/Blueprints/Units/Characters/BP_CharacterBase.isAI` _asbp_character_base) (`/Game/TurnBasedStrategyRPGTemplate/Blueprints/Units/Characters/BP_CharacterBase.isAI` character)) _asbp_character_base))))
    (:`CastFailed`
      (return false null))))

(fn `IsEmpty`
  (returns (isFree :type Boolean))
  ;[1 1 1] Checks if the slot is empty
  (return (== (`self.containedUnit`) null)))

(fn `IsEnemySlot`
  (params (character :type "/Game/TurnBasedStrategyRPGTemplate/Blueprints/Units/Characters/BP_CharacterBase Object Reference"))
  (returns (isEnemySlot :type Boolean) (enemyCharacter :type "/Game/TurnBasedStrategyRPGTemplate/Blueprints/Units/Characters/BP_CharacterBase Object Reference"))
  ;[1 1 1] Check if the slot contains enemy unit
  (bind _asbp_character_base (cast `/Game/TurnBasedStrategyRPGTemplate/Blueprints/Units/Characters/BP_CharacterBase` (`self.containedUnit`))
    (:`then`
      (bind _isdead (`/Game/TurnBasedStrategyRPGTemplate/Blueprints/Units/Characters/BP_CharacterBase.IsDead` _asbp_character_base))
      (if _isdead
        (return false null)
        (else
          (return (!= (`/Game/TurnBasedStrategyRPGTemplate/Blueprints/Units/Characters/BP_CharacterBase.isAI` _asbp_character_base) (`/Game/TurnBasedStrategyRPGTemplate/Blueprints/Units/Characters/BP_CharacterBase.isAI` character)) _asbp_character_base))))
    (:`CastFailed`
      (return false null))))

(fn `UserConstructionScript`)